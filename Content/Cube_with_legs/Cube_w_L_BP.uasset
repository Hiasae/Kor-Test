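; Enemy cube-with-legs actor that chases the player, attacks in melee range and dies when its health drops below zero.
; Tick drives the capsule forward by physics velocity, smoothly yaws toward the player, and stops to attack when squared distance falls below Attackrange.
; Damage is applied whenever the polled DMGnotify value from its Anim Blueprint changes, syncing hits to the animation.
; FirstPersonProjectile capsule hits reduce its health.
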(event `self.ReceiveTick`
  (params (DeltaSeconds :type "Float (single-precision)"))
  (bind _returnvalue (`self.K2_GetActorLocation`))
  (bind _returnvalue_2 (`self.K2_GetActorLocation` (`GameplayStatics.GetPlayerPawn` 0)))
  ;[1 1 1] Simple Forward Motion
  (`PrimitiveComponent.SetPhysicsLinearVelocity` (`self.CapsuleComponent`) (* (`self.GetActorForwardVector`) (`self.Velocity`)) false "None")
  ;[1 1 1] Rotate towards Player
  (`self.K2_SetActorRotation` (`KismetMathLibrary.MakeRotator` 0.0 0.0 (.yaw (`KismetMathLibrary.RInterpTo` (`self.K2_GetActorRotation`) (`KismetMathLibrary.FindLookAtRotation` _returnvalue _returnvalue_2) DeltaSeconds 2.0))))
  ;[1 1 1] Attack
  (if (< (`KismetMathLibrary.VSizeSquared` (- _returnvalue _returnvalue_2)) (`self.Attackrange`))
    (set `self.Attacking` true)
    (set `self.Velocity` 0.0)
    (bind _ascube_w_l_animbp (cast `/Game/Cube_with_Legs/Cube_w_L_ANIMBP` (`SkeletalMeshComponent.GetAnimInstance` (`self.Enemy_Cube_with_Legs`))))
    (bind _dmgnotify (`/Game/Cube_with_Legs/Cube_w_L_ANIMBP.DMGnotify` _ascube_w_l_animbp))
    ;[1 1 1] Check if Damage Notifier on Animation is changed (means activated )
    (if (!= (`self.DMGnotify`) _dmgnotify)
      (set `self.DMGnotify` _dmgnotify)
      (`GameplayStatics.ApplyDamage` (`GameplayStatics.GetPlayerPawn` 0) 10.0)
      (if (> 0.0 (`self.Health`)) :!label _label
        (`self.K2_DestroyActor`)))
    (else
      (`KismetSystemLibrary.Delay` 0.2)
      (set `self.Attacking` false)
      (set `self.Velocity` 200.0)
      (goto _label))))

(event `self.CapsuleComponent.OnComponentHit`
  (params (HitComponent :type "PrimitiveComponent Object Reference") (OtherActor :type "Actor Object Reference") (OtherComp :type "PrimitiveComponent Object Reference") (NormalImpulse :type "Vector Structure") (Hit :type "HitResult Structure (by ref)"))
  ;[1 1 1] If FirstPersonProjectile Hits Damage this Actor
  (cast `/Game/FirstPersonBP/Blueprints/FirstPersonProjectile` OtherActor)
  (set `self.Health` (- (`self.Health`) 11.0)))

(fn `UserConstructionScript`)